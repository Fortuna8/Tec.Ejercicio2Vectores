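; BP_Orco is an orc actor that moves straight toward the referenced archer, ArqueroReferencia, every tick.
; Tick adds the normalized direction scaled by VelocidadOrco without delta time or sweep, so movement is frame-rate dependent and ignores collision.
; BeginPlay draws a long-lasting green debug box at the starting location.
; The construction script creates dynamic materials on two cylinders and a sphere, tinting them with ColorOrco.
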(event EventBeginPlay
  (Rendering|Debug|DrawDebugBox (Transformation|GetActorLocation) "50.000000,50.000000,50.000000" "(R=0.196835,G=1.000000,B=0.248990,A=1.000000)" "0, 0, 0" 3.6e+03 1e+01))

(event EventTick
  (params (DeltaSeconds :type Float%20%28single-precision%29))
  (Transformation|AddActorWorldOffset (* (Math|Vector|Normalize (- (Transformation|GetActorLocation (Variables|Default|GetarqueroReferencia)) (Transformation|GetActorLocation))) (Variables|Default|GetvelocidadOrco))))

(fn ConstructionScript
  (bind _returnvalue (Rendering|Material|CreateDynamicMaterialInstance (Variables|Default|GetCylinder1) 0 0 "None" :!class /Script/Engine.PrimitiveComponent))
  (bind _returnvalue_2 (Rendering|Material|CreateDynamicMaterialInstance (Variables|Default|GetCylinder) 0 "/Game/Blueprints/Ejercicio2/OrcoSkinMaterial.OrcoSkinMaterial" "None" :!class /Script/Engine.PrimitiveComponent))
  (bind _returnvalue_3 (Rendering|Material|CreateDynamicMaterialInstance (Variables|Default|GetSphere) 0 0 "None" :!class /Script/Engine.PrimitiveComponent))
  (Rendering|Material|SetVectorParameterValue _returnvalue "colorOrco" (Variables|Default|GetcolorOrco) :!class /Script/Engine.MaterialInstanceDynamic))